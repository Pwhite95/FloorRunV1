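; FloorRunGameBP runs the round countdown for a floor-run game and decides whether the environment is completed.
; On BeginPlay, if the ColoredHall1 streaming level is loaded, a looping one-second timer starts after a delay and calls GameTimer to decrement Minutes and Seconds.
; At zero, no remaining InteractionCount sets EnviromentComplete; otherwise it prints "Restart" and shows "Done" on Check_Total's text.
; FloorRunSaveGame create, load and write chains exist but are unconnected.
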(event `self.ReceiveTick`
  (params (DeltaSeconds :type "Float (single-precision)")))

(event `self.ReceiveBeginPlay`
  (if (`LevelStreaming.IsLevelLoaded` (`GameplayStatics.GetStreamingLevel` "ColoredHall1"))
    (`KismetSystemLibrary.K2_SetTimer` null "GameTimer" 1.0 true 5.0)))

(event `ReadSG`)

(event `WritetoSG`
  ;[1 1 1] Write SG
)

(fn `GameTimer`
  ;[1 1 1] Game Timer
  (set `self.Seconds` (- (`self.Seconds`) 1))
  (if (< (`self.Seconds`) 0)
    (set `self.Minutes` (- (`self.Minutes`) 1))
    (set `self.Seconds` 59))
  (if (== (`self.Seconds`) 0)
    (if (== (`self.Minutes`) 0)
      (if (== (`self.Interaction Count`) 0)
        (`KismetSystemLibrary.PrintString` "Complete")
        (set `self.Enviroment Complete` 1)
        (else
          (`KismetSystemLibrary.PrintString` "Restart")
          (bind _returnvalue (`GameplayStatics.GetActorOfClass` "/Game/VirtualRealityBP/Blueprints/Check/Check_Total.Check_Total_C"))
          (`TextRenderComponent.K2_SetText` (`/Game/VirtualRealityBP/Blueprints/Check/Check_Total.TextRender` _returnvalue) (`KismetTextLibrary.Conv_StringToText` "Done")))))))

(fn `UserConstructionScript`)